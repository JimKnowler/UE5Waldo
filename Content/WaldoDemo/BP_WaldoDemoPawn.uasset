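; BP_WaldoDemoPawn is a demo pawn that drives a skeletal mesh's animation from a Waldo input device connected over a serial port.
; On BeginPlay it switches the view to a tagged cine camera and binds to Waldo's mouth input and frame-end events.
; Mouth values are normalized from a 0–255 range into WaldoState, which is copied to the animation Blueprint on each Waldo frame end.
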(event `self.ReceiveBeginPlay`
  (`self.BeginPlay_Camera`)
  (`WaldoComponent.BindDelegateForInput` (`self.Waldo`) "mouth" (`|CreateDelegate` :!event `Event OnInputValueMouth`))
  (add `WaldoComponent.OnFrameEnd` (`self.Waldo`) (delegate `Event OnFrameEnd`)))

(event `Event OnFrameEnd`
  (bind _asbp_waldo_demo_anim_blueprint (cast `/Game/WaldoDemo/BP_WaldoDemoAnimBlueprint` (`SkeletalMeshComponent.GetAnimInstance` (`self.SkeletalMesh`))))
  (set `/Game/WaldoDemo/BP_WaldoDemoAnimBlueprint.WaldoState` (`self.WaldoState`) _asbp_waldo_demo_anim_blueprint))

(event `Event OnInputValueMouth`
  (params (Value :type Integer))
  (setmembers `/Game/WaldoDemo/WaldoState` :`StructRef` (`self.WaldoState`) :`mouth` (/ (`KismetMathLibrary.Conv_IntToDouble` Value) 255.0)))

(fn `BeginPlay_Camera`
  (bind _outactors (`GameplayStatics.GetAllActorsOfClassWithTag` "/Script/CinematicCamera.CineCameraActor" "camera"))
  (`PlayerController.SetViewTargetWithBlend` (`GameplayStatics.GetPlayerController` 0) (`|GetArrayItem` _outactors) 0.0 "VTBlend_Linear" 0.0 false))

(fn `Connect`
  (params (SerialPortDevice :type "SerialPortDevice Structure"))
  (bind _returnvalue (`WaldoComponent.Connect` (`self.Waldo`) SerialPortDevice 9600))
  (`KismetSystemLibrary.PrintText` (`KismetMathLibrary.SelectText` "Successfully connected to Waldo" "Failed to connect to waldo" _returnvalue)))

(fn `UserConstructionScript`)